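; Escape-room game controller that drives objective progression and mirrors it in the player's HUD.
; It binds to laser receivers on observed nodes; each node's index selects a one-shot objective change and progress flag, then that receiver is unbound.
; One-shot trigger boxes add hints as the player arrives, some gated by those flags.
; ObjectivesManager events create, update or remove HUD list widgets with fade animations, tracked in a name-keyed map.
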(event `OnLaserBeamReceived_Event`
  (params (LaserBeamReceivedActor :type "Actor Object Reference"))
  (bind _observedlasernodes (`self.ObservedLaserNodes`))
  (bind _returnvalue (`KismetArrayLibrary.Array_Find` _observedlasernodes LaserBeamReceivedActor))
  (bind _returnvalue_2 (`self.GetComponentByClass` (`|GetArrayItem` _observedlasernodes _returnvalue) "/Script/Escape.LaserBeamReceiver"))
  (switch `int` _returnvalue
    (:`0`
      (`/Engine/EditorBlueprintResources/StandardMacros.DoOnce` false
        (:`Completed`
          (`ObjectivesManager.RemoveObjective` (`self.ObjectivesManager`) "SimonObjective"))))
    (:`1`
      (`/Engine/EditorBlueprintResources/StandardMacros.DoOnce` false
        (:`Completed`
          (`ObjectivesManager.AddObjective` (`self.ObjectivesManager`) "TableObjective" "There is something about this model town...")
          (set `self.TableLaseractive` true))))
    (:`2`
      (`/Engine/EditorBlueprintResources/StandardMacros.DoOnce` false
        (:`Completed`
          (`ObjectivesManager.AddObjective` (`self.ObjectivesManager`) "MainGoal" "Get the Key!")
          (`ObjectivesManager.RemoveObjective` (`self.ObjectivesManager`) "TableObjective")
          (set `self.DoorOpen` true)))))
  (if (`KismetSystemLibrary.IsValid` _returnvalue_2)
    (remove `LaserBeamReceiver.OnLaserBeamReceived` _returnvalue_2 (delegate `OnLaserBeamReceived_Event`))))

(event `self.ReceiveBeginPlay`
  (`KismetSystemLibrary.Delay` 0.5)
  (`ObjectivesManager.AddObjective` (`self.ObjectivesManager`) "MainGoal" "Get to the Key.")
  (`ObjectivesManager.AddObjective` (`self.ObjectivesManager`) "SimonObjective" "Look around...")
  (for _array_element (`self.ObservedLaserNodes`)
    (bind _returnvalue (`self.GetComponentByClass` _array_element "/Script/Escape.LaserBeamReceiver"))
    (if (`KismetSystemLibrary.IsValid` _returnvalue)
      (add `LaserBeamReceiver.OnLaserBeamReceived` _returnvalue (delegate `OnLaserBeamReceived_Event`)))))

(event `self.ObjectivesManager.OnAddObjectiveToHUD`
  (params (ObjectiveName :type String) (ObjectiveText :type String))
  ;[1 1 1] Add New Objective to HUD
  (bind _objectivewidget (`self.AddNewObjectiveItemWidget` ObjectiveText))
  (`BlueprintMapLibrary.Map_Add` (`self.CurrentObjectiveDisplay`) ObjectiveName _objectivewidget)
  (`UserWidget.PlayAnimation` _objectivewidget (`/Game/EscapeCustomAssets/UI/ObjectiveItem.ObjectiveItemFadeIn` _objectivewidget) 0.0 1 "Forward" 1.0))

(event `self.ObjectivesManager.OnUpdateObjectiveInHUD`
  (params (ObjectiveName :type String) (ObjectiveText :type String))
  (bind (_value _returnvalue) (`BlueprintMapLibrary.Map_Find` (`self.CurrentObjectiveDisplay`) ObjectiveName))
  ;[1 1 1] Update Objective in HUD
  (if _returnvalue
    (`UserWidget.PlayAnimation` _value (`/Game/EscapeCustomAssets/UI/ObjectiveItem.ObjectiveItemFadeOut` _value) 0.0 1 "Forward" 1.0)
    (`KismetSystemLibrary.Delay` 1.0)
    (set `/Game/EscapeCustomAssets/UI/ObjectiveItem.ObjectiveItemText` ObjectiveText _value)
    (`UserWidget.PlayAnimation` _value (`/Game/EscapeCustomAssets/UI/ObjectiveItem.ObjectiveItemFadeIn` _value) 0.0 1 "Forward" 1.0)))

(event `self.ObjectivesManager.OnRemoveObjectiveFromHUD`
  (params (ObjectiveName :type String))
  (bind (_value _returnvalue) (`BlueprintMapLibrary.Map_Find` (`self.CurrentObjectiveDisplay`) ObjectiveName))
  ;[1 1 1] Remove Objective from HUD
  (if _returnvalue
    (`UserWidget.PlayAnimation` _value (`/Game/EscapeCustomAssets/UI/ObjectiveItem.ObjectiveItemFadeOut` _value) 0.0 1 "Forward" 1.0)
    (`KismetSystemLibrary.Delay` 1.0)
    (bind _returnvalue_2 (`PanelWidget.RemoveChild` (`self.HUD_ObjectivesList`) _value))
    (if _returnvalue_2
      (`BlueprintMapLibrary.Map_Remove` (`self.CurrentObjectiveDisplay`) ObjectiveName))))

(event `self.SimonGameObjectiveTriggerBox.OnActorBeginOverlap`
  (params (OverlappedActor :type "Actor Object Reference") (OtherActor :type "Actor Object Reference"))
  (cast `/Game/EscapeCustomAssets/Blueprints/FP_character_Adv` OtherActor)
  (if true
    (`/Engine/EditorBlueprintResources/StandardMacros.DoOnce` false
      (:`Completed`
        (`ObjectivesManager.AddObjective` (`self.ObjectivesManager`) "SimonObjective" "Harmonzie the Orbs.")))))

(event `self.GetTheDoorOpenTriggerBox.OnActorBeginOverlap`
  (params (OverlappedActor :type "Actor Object Reference") (OtherActor :type "Actor Object Reference"))
  (cast `/Game/EscapeCustomAssets/Blueprints/FP_character_Adv` OtherActor)
  (if true
    (`/Engine/EditorBlueprintResources/StandardMacros.DoOnce` false
      (:`Completed`
        (if (not (`self.DoorOpen`))
          (`ObjectivesManager.AddObjective` (`self.ObjectivesManager`) "MainGoal" "Open the door to the Key."))))))

(event `self.GetTheKeyTriggerBox.OnActorBeginOverlap`
  (params (OverlappedActor :type "Actor Object Reference") (OtherActor :type "Actor Object Reference"))
  (cast `/Game/EscapeCustomAssets/Blueprints/FP_character_Adv` OtherActor)
  (if true
    (`/Engine/EditorBlueprintResources/StandardMacros.DoOnce` false
      (:`Completed`
        (if (not (`self.DoorOpen`))
          (`ObjectivesManager.AddObjective` (`self.ObjectivesManager`) "MainGoal" "How did you get here?!"))))))

(event `self.TableTriggerBox.OnActorBeginOverlap`
  (params (OverlappedActor :type "Actor Object Reference") (OtherActor :type "Actor Object Reference"))
  (cast `/Game/EscapeCustomAssets/Blueprints/FP_character_Adv` OtherActor)
  (if true
    (`/Engine/EditorBlueprintResources/StandardMacros.DoOnce` false
      (:`Completed`
        (if (not (`self.TableLaseractive`))
          (`ObjectivesManager.AddObjective` (`self.ObjectivesManager`) "TableObjective" "There is something about this model town... but it's not working (yet)."))))))

(fn `AddNewObjectiveItemWidget`
  (params (ObjectiveText :type String))
  (returns (ObjectiveWidget :type "/Game/EscapeCustomAssets/UI/ObjectiveItem Object Reference"))
  (bind _returnvalue (`GameplayStatics.GetPlayerController` 0))
  (bind _returnvalue_2 (`|CreateWidget` "/Game/EscapeCustomAssets/UI/ObjectiveItem.ObjectiveItem_C" _returnvalue))
  (set `/Game/EscapeCustomAssets/UI/ObjectiveItem.ObjectiveItemText` ObjectiveText _returnvalue_2)
  (bind _asescape_hud (cast `/Game/EscapeCustomAssets/UI/EscapeHUD` (`PlayerController.GetHUD` _returnvalue)))
  (bind _output_get (set `self.HUD_ObjectivesList` (`/Game/EscapeCustomAssets/UI/HUDInfo.ObjectivesList` (`/Game/EscapeCustomAssets/UI/EscapeHUD.HUD_InfoWidget` _asescape_hud))))
  (`PanelWidget.AddChild` _output_get _returnvalue_2)
  (return _returnvalue_2))

(fn `UserConstructionScript`)