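; Front door exit actor that ends the game with a win when its switch is activated while unlocked.
; It clears all widgets and shows the Outro screen, then after a short delay plays a fade-out level sequence.
; Shortly before the sequence ends, it opens the MenuLevel to return to the main menu.
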(event `self.Switch.OnSwitchActivation`
  (params (ActivatedSwtichActor :type "Actor Object Reference"))
  (bind _sequenceplayer (`LevelSequenceActor.SequencePlayer` (`self.FadeOutSequence`)))
  ;[1 1 1] Show Win Screen and return to Main Menu
  (if (not (`self.Locked`))
    (`WidgetLayoutLibrary.RemoveAllWidgets`)
    (bind _returnvalue (`|CreateWidget` "/Game/EscapeCustomAssets/UI/Outro.Outro_C" (`GameplayStatics.GetPlayerController` 0)))
    (`UserWidget.AddToViewport` _returnvalue 0)
    (`KismetSystemLibrary.Delay` 3.5)
    (`MovieSceneSequencePlayer.Play` _sequenceplayer)
    (`KismetSystemLibrary.Delay` (- (`TimeManagementBlueprintLibrary.Conv_QualifiedFrameTimeToSeconds` (`MovieSceneSequencePlayer.GetDuration` _sequenceplayer)) 3.0))
    (`GameplayStatics.OpenLevel` "MenuLevel")))

(fn `UserConstructionScript`)