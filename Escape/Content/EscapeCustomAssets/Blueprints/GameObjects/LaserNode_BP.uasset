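; LaserNode is a clickable node in a table laser game that forwards clicks to its TableGameLaserController component and lights up while activated.
; On BeginPlay it aims the laser emitter at an optional initial target and places a point light in front of it.
; Tick plays or reverses a timeline, rate-matched to the controller's activation delay, that fades the light up to its construction-time intensity and triggers the node sound.
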(event `self.ReceiveBeginPlay`
  (bind _returnvalue (`SceneComponent.GetRelativeTransform` (`self.LaserBeamEmitter`)))
  (if (`KismetSystemLibrary.IsValid` (`self.OptionalInitialTarget`))
    ;[1 1 1] Point Laser Emitter at Target
    (`SceneComponent.K2_SetWorldRotation` (`self.LaserBeamEmitter`) (`KismetMathLibrary.FindLookAtRotation` (`SceneComponent.K2_GetComponentLocation` (`self.LaserBeamEmitter`)) (`self.K2_GetActorLocation` (`self.OptionalInitialTarget`))) false false))
  ;[1 1 1] Place Pointlight in front of Laser Emitter
  (`SceneComponent.K2_SetRelativeLocation` (`self.PointLight`) (+ (`KismetMathLibrary.GreaterGreater_VectorRotator` (`self.LightDistanceVector`) (`KismetMathLibrary.TransformRotation` _returnvalue)) (`KismetMathLibrary.TransformLocation` _returnvalue)) false true)
  (`TimelineComponent.SetPlayRate` (`self.LightActivation`) (/ 1.0 (`TableGameLaserController.ActivationDelay` (`self.TableGameLaserController`)))))

(event `self.ReceiveActorOnClicked`
  (params (ButtonPressed :type "Key Structure"))
  (`ActivationReceiver.OnClick` (`self.TableGameLaserController`)))

(event `self.ReceiveTick`
  (params (DeltaSeconds :type "Float (single-precision)"))
  ;[1 1 1] Point Light On/Off Controle
  (if (> (`TableGameLaserController.CurrentActivationDuration` (`self.TableGameLaserController`)) 0.0)
    (bind (_direction _lightintensity) (`Timeline|LightActivation` :!label _label)
      (:`Update`
        (`LightComponent.SetIntensity` (`self.PointLight`) (* _lightintensity (`self.MaxLightIntensity`))))
      (:`SoundActivation`
        (if (> (`TableGameLaserController.CurrentActivationDuration` (`self.TableGameLaserController`)) 0.0)
          (`AudioComponent.Play` (`self.NodeSound`) 0.0))))
    (else
      (goto _label :!via `Reverse`))))

(fn `UserConstructionScript`
  (set `self.MaxLightIntensity` (`LightComponentBase.Intensity` (`self.PointLight`))))