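; Radio actor Blueprint with looping music that a switch toggles on and off.
; Shortly after BeginPlay, the music starts at a random point in the loop so it does not begin from the top.
; Switch activation flips the Playing state, and a timeline fades the volume in or out by scaling the volume multiplier rather than stopping playback.
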(event `self.ReceiveBeginPlay`
  (`KismetSystemLibrary.Delay` 0.01)
  (`AudioComponent.Play` (`self.RadioMusic`) (`KismetMathLibrary.RandomFloatInRange` 0.0 (`self.SoundLoopDuration`)))
  (if (`self.Playing`) :!label _label
    (bind (_direction _volume) (`Timeline|VolumeTimeLine` :!label _label_2)
      (:`Update`
        (`AudioComponent.SetVolumeMultiplier` (`self.RadioMusic`) (* _volume (`self.Volume`)))))
    (else
      (goto _label_2 :!via `Reverse`))))

(event `self.Switch.OnSwitchActivation`
  (params (ActivatedSwtichActor :type "Actor Object Reference"))
  (set `self.Playing` (not (`self.Playing`)))
  (goto _label))

(fn `UserConstructionScript`)