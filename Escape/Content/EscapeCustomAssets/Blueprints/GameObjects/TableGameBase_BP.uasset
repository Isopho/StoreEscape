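; TableGameBase_BP is the base table game Blueprint, moving the first-person player into a mouse-driven table view and back out.
; An activation request from TableGameController locks move and look, blends the camera to the table and switches cursor, input mode and highlight method.
; If the start laser node is active, an intro sequence plays once before that blend.
; Right mouse button blends back to the character and restores controls and crosshair.
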(event `self.TableGameController.OnActivateGameRequest`
  (bind _returnvalue (`GameplayStatics.GetPlayerController` 0))
  (bind _returnvalue_2 (`GameplayStatics.GetPlayerController` 0))
  (bind _startlasernode (`self.StartlaserNode`))
  (bind _returnvalue_3 (`self.GetComponentByClass` _startlasernode "/Script/Escape.TableGameLaserController"))
  (bind _sequenceplayer (`LevelSequenceActor.SequencePlayer` (`self.IntroSequence`)))
  ;[1 1 1] Enter Table View Mode
  (bind _asfp_controller_adv (cast `/Game/EscapeCustomAssets/Blueprints/FP_Controller_Adv` (`GameplayStatics.GetPlayerController` 0)))
  (`/Game/EscapeCustomAssets/Blueprints/FP_Controller_Adv.RemoveCrossAir` _asfp_controller_adv)
  (`Controller.SetIgnoreMoveInput` _returnvalue_2 true)
  (`Controller.SetIgnoreLookInput` _returnvalue_2 true)
  (if (`self.PlayIntro`)
    ;[1 1 1] Check if TableGame is active (Start Laser node activated)
    (if (`KismetSystemLibrary.IsValid` _startlasernode)
      (if (`KismetSystemLibrary.IsValid` _returnvalue_3)
        (if (> (`TableGameLaserController.CurrentActivationDuration` _returnvalue_3) 0.0)
          ;[1 1 1] Play Table Game Intro
          (`PlayerController.SetViewTargetWithBlend` (`GameplayStatics.GetPlayerController` 0) (`self.IntoSequenceCamera`) (`self.TransitionDuration`) "VTBlend_EaseInOut" 3.0 false)
          (`KismetSystemLibrary.Delay` (- (`self.TransitionDuration`) 1.0))
          (`MovieSceneSequencePlayer.Play` _sequenceplayer)
          (`KismetSystemLibrary.Delay` (- (`TimeManagementBlueprintLibrary.Conv_QualifiedFrameTimeToSeconds` (`MovieSceneSequencePlayer.GetDuration` _sequenceplayer)) 1.0))
          (`MovieSceneSequencePlayer.Pause` _sequenceplayer)
          (set `self.PlayIntro` false) ; Play Intro only once
        ))))
  ;;[1 1 1] Blend to Table Camera
  (`PlayerController.SetViewTargetWithBlend` (`GameplayStatics.GetPlayerController` 0) self (`self.TransitionDuration`) "VTBlend_EaseInOut" 3.0 false)
  (`KismetSystemLibrary.Delay` (`self.TransitionDuration`))
  (`self.EnableInput` _returnvalue)
  (set `PlayerController.bShowMouseCursor` true _returnvalue)
  (bind _asfp_controller_adv_2 (cast `/Game/EscapeCustomAssets/Blueprints/FP_Controller_Adv` (`GameplayStatics.GetPlayerController` 0)))
  (`/Game/EscapeCustomAssets/Blueprints/FP_Controller_Adv.OnSwitchHighlightMethod` _asfp_controller_adv_2 "NewEnumerator0") ; Contains 1 Second Delay
  (set `self.InTableView` true)
  (`WidgetBlueprintLibrary.SetInputMode_GameAndUIEx` (`GameplayStatics.GetPlayerController` 0) null "DoNotLock" false))

(event `Key|RightMouseButton`
  (params (Key :type "Key Structure"))
  (bind _returnvalue (`GameplayStatics.GetPlayerController` 0))
  ;[1 1 1] Exit Table View Mode
  (:`Pressed`
    (if (`self.InTableView`)
      (set `self.InTableView` false)
      (set `PlayerController.bShowMouseCursor` false (`GameplayStatics.GetPlayerController` 0))
      (`self.DisableInput` (`GameplayStatics.GetPlayerController` 0))
      (`WidgetBlueprintLibrary.SetInputMode_GameOnly` (`GameplayStatics.GetPlayerController` 0))
      (`PlayerController.SetViewTargetWithBlend` (`GameplayStatics.GetPlayerController` 0) (`GameplayStatics.GetPlayerCharacter` 0) (`self.TransitionDuration`) "VTBlend_EaseInOut" 3.0 false)
      (bind _asfp_controller_adv (cast `/Game/EscapeCustomAssets/Blueprints/FP_Controller_Adv` (`GameplayStatics.GetPlayerController` 0)))
      (`/Game/EscapeCustomAssets/Blueprints/FP_Controller_Adv.OnSwitchHighlightMethod` _asfp_controller_adv "NewEnumerator1") ; Contains 1 Second Delay
      (`KismetSystemLibrary.Delay` (- (`self.TransitionDuration`) 0.7))
      (`Controller.ResetIgnoreMoveInput` _returnvalue)
      (`Controller.ResetIgnoreLookInput` _returnvalue)
      (bind _asfp_controller_adv_2 (cast `/Game/EscapeCustomAssets/Blueprints/FP_Controller_Adv` (`GameplayStatics.GetPlayerController` 0)))
      (`/Game/EscapeCustomAssets/Blueprints/FP_Controller_Adv.AddCrossAir` _asfp_controller_adv_2))))

(fn `UserConstructionScript`)