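; Starter laser node for the table laser game, deriving from a parent Blueprint that supplies its construction logic.
; On BeginPlay it disables the LaserBeam component's tick if the laser is blocked.
; When TableGameLaserController fires its switch activation with a positive current activation duration, the node clears the blocked flag and re-enables beam ticking.
; The graph contains no logic to block the beam again.
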(event `self.TableGameLaserController.OnSwitchActivation`
  (params (ActivatedSwtichActor :type "Actor Object Reference"))
  (if (> (`TableGameLaserController.CurrentActivationDuration` (`self.TableGameLaserController`)) 0.0)
    (set `self.LaserBlocked` false)
    (`ActorComponent.SetComponentTickEnabled` (`self.LaserBeam`) true)))

(event `self.ReceiveBeginPlay`
  (if (`self.LaserBlocked`)
    (`ActorComponent.SetComponentTickEnabled` (`self.LaserBeam`) false)))

(fn `UserConstructionScript`
  (`parent.UserConstructionScript`))