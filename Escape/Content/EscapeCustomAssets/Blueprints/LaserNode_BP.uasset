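; LaserNode_BP is a clickable laser node actor for a table laser game, with click handling delegated to its TableGameLaserController.
; On BeginPlay it aims its beam emitter at an optional initial target.
; Each Tick it plays the LightActivation timeline forward while the controller's activation duration is positive, otherwise reverses it, with play rate derived from the activation delay.
; The timeline scales the point light up to the intensity cached at construction.
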(event `self.ReceiveBeginPlay`
  (if (`KismetSystemLibrary.IsValid` (`self.OptionalInitialTarget`))
    (`SceneComponent.K2_SetWorldRotation` (`self.LaserBeamEmitter`) (`KismetMathLibrary.FindLookAtRotation` (`SceneComponent.K2_GetComponentLocation` (`self.LaserBeamEmitter`)) (`self.K2_GetActorLocation` (`self.OptionalInitialTarget`))) false false)))

(event `self.ReceiveActorOnClicked`
  (params (ButtonPressed :type "Key Structure"))
  (`ActivationReceiver.OnClick` (`self.TableGameLaserController`)))

(event `self.ReceiveTick`
  (params (DeltaSeconds :type "Float (single-precision)"))
  (`TimelineComponent.SetPlayRate` (`self.LightActivation`) (/ 1.0 (`TableGameLaserController.ActivationDelay` (`self.TableGameLaserController`))))
  (if (> (`TableGameLaserController.CurrentActivationDuration` (`self.TableGameLaserController`)) 0.0)
    (bind (_direction _lightintensity) (`Timeline|LightActivation` :!label _label)
      (:`Update`
        (`LightComponent.SetIntensity` (`self.PointLight`) (* _lightintensity (`self.MaxLightIntensity`)))))
    (else
      (goto _label :!via `Reverse`))))

(fn `UserConstructionScript`
  (set `self.MaxLightIntensity` (`LightComponentBase.Intensity` (`self.PointLight`))))