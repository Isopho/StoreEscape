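; Simon orb actor that lights up and plays a sound in response to SimonOrbController flare and glow requests.
; Flare requests drive a timeline that scales light intensity and volume by the requested values, with play rate set from duration.
; Glow requests chain a faster start timeline into a continuous glow timeline, playing sound at base volume.
; Stop requests only halt the continuous glow timeline, without resetting light or sound.
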(event `self.SimonOrbController.FlareOrbRequest`
  (params (Duration :type "Float (single-precision)") (LightIntensity :type "Float (single-precision)") (VolumeMultiplyer :type "Float (single-precision)"))
  (bind _orbsound (`self.OrbSound`))
  ;[1 1 1] OrbFlare
  (`TimelineComponent.SetPlayRate` (`self.LightFlare`) (/ 1.0 Duration))
  (bind (_direction _lightintensityproportion) (`Timeline|LightFlare` :!via `PlayFromStart`)
    (:`Update`
      (`LightComponent.SetIntensity` (`self.OrbLight`) (* _lightintensityproportion LightIntensity))
      (`AudioComponent.SetVolumeMultiplier` _orbsound (* _lightintensityproportion VolumeMultiplyer (`self.BaseVolumeMultiplier`))))
    (:`OrbSoundStart`
      (`AudioComponent.Play` _orbsound 0.0))))

(event `self.SimonOrbController.StartOrbGlowRequest`
  (params (Duration :type "Float (single-precision)"))
  ;[1 1 1] OrbGlow
  (`TimelineComponent.SetPlayRate` (`self.ContinuousGlow`) (/ 1.0 Duration))
  (`TimelineComponent.SetPlayRate` (`self.StartGlow`) (/ 10.0 Duration))
  (bind (_direction _lightintensityproportion) (`Timeline|StartGlow` :!via `PlayFromStart`)
    (:`Update`
      (`LightComponent.SetIntensity` (`self.OrbLight`) (* _lightintensityproportion (`self.MaxGlowIntensity`))))
    (:`Finished`
      (bind (_direction_2 _lightintensityproportion_2) (`Timeline|ContinuousGlow` :!label _label)
        (:`Update`
          (`LightComponent.SetIntensity` (`self.OrbLight`) (* _lightintensityproportion_2 (`self.MaxGlowIntensity`))))))
    (:`StartingGlow`
      (`AudioComponent.SetVolumeMultiplier` (`self.OrbSound`) (`self.BaseVolumeMultiplier`))
      (`AudioComponent.Play` (`self.OrbSound`) 0.0))))

(event `self.SimonOrbController.StopOrbGlowRequest`
  ;[1 1 1] OrbGlow
  (goto _label :!via `Stop`))

(fn `UserConstructionScript`)