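; Start camera actor that takes over the player's view at BeginPlay and can play an intro transition into gameplay.
; With PlayIntro set, it locks move and look input, pauses briefly, then eases the view to the player character over IntroBlendTime.
; Input returns shortly before the blend ends.
; Without PlayIntro, the view stays on this actor; a disconnected PauseGame call never runs.
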(event `self.ReceiveBeginPlay`
  (bind _returnvalue (`GameplayStatics.GetPlayerController` 0))
  (bind _returnvalue_2 (`GameplayStatics.GetPlayerController` 0))
  (`PlayerController.SetViewTargetWithBlend` (`GameplayStatics.GetPlayerController` 0) self 0.0 "VTBlend_Linear" 0.0 false)
  (if (`self.PlayIntro`)
    (`Controller.SetIgnoreMoveInput` _returnvalue true)
    (`Controller.SetIgnoreLookInput` _returnvalue true)
    (`KismetSystemLibrary.Delay` 1.0)
    (`PlayerController.SetViewTargetWithBlend` (`GameplayStatics.GetPlayerController` 0) (`GameplayStatics.GetPlayerCharacter` 0) (`self.IntroBlendTime`) "VTBlend_EaseInOut" 3.0 false)
    (`KismetSystemLibrary.Delay` (- (`self.IntroBlendTime`) 0.5))
    (`Controller.SetIgnoreMoveInput` _returnvalue_2 false)
    (`Controller.SetIgnoreLookInput` _returnvalue_2 false)))

(fn `UserConstructionScript`)