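; TableGameBase is a base actor for table games that switches the player between normal play and a focused game view.
; Its TableGameController's activation request blends the view to this actor, locks player movement and look, then enables the actor's input after the transition.
; Right mouse disables that input, blends back to the character, and restores movement and look once the same TransitionDuration elapses.
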(event `self.TableGameController.OnActivateGameRequest`
  (bind _returnvalue (`GameplayStatics.GetPlayerController` 0))
  ;[1 1 1] Enter TableGameMode
  (`PlayerController.SetViewTargetWithBlend` (`GameplayStatics.GetPlayerController` 0) self (`self.TransitionDuration`) "VTBlend_EaseInOut" 3.0 false)
  (`Controller.SetIgnoreMoveInput` _returnvalue true)
  (`Controller.SetIgnoreLookInput` _returnvalue true)
  (`KismetSystemLibrary.Delay` (`self.TransitionDuration`))
  (`self.EnableInput` (`GameplayStatics.GetPlayerController` 0)))

(event `Key|RightMouseButton`
  (params (Key :type "Key Structure"))
  (bind _returnvalue (`GameplayStatics.GetPlayerController` 0))
  ;[1 1 1] Exit TableGameMode
  (:`Pressed`
    (`self.DisableInput` (`GameplayStatics.GetPlayerController` 0))
    (`PlayerController.SetViewTargetWithBlend` (`GameplayStatics.GetPlayerController` 0) (`GameplayStatics.GetPlayerCharacter` 0) (`self.TransitionDuration`) "VTBlend_EaseInOut" 3.0 false)
    (`KismetSystemLibrary.Delay` (`self.TransitionDuration`))
    (`Controller.ResetIgnoreMoveInput` _returnvalue)
    (`Controller.ResetIgnoreLookInput` _returnvalue)))

(fn `UserConstructionScript`)