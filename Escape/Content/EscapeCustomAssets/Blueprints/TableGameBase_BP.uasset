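; Base Blueprint for a table game that switches the player from first-person play into a cursor-driven table view.
; On the TableGameController's activate request, it locks move and look, blends the view to itself, enables input and switches the highlight method.
; A sequence camera intro plays first, once, if the start laser node has a positive activation duration.
; Right mouse blends back to the character and restores the controls.
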(event `self.TableGameController.OnActivateGameRequest`
  (bind _returnvalue (`GameplayStatics.GetPlayerController` 0))
  (bind _returnvalue_2 (`GameplayStatics.GetPlayerController` 0))
  (bind _startlasernode (`self.StartlaserNode`))
  (bind _introsequence (`self.IntroSequence`))
  (bind _returnvalue_3 (`self.GetComponentByClass` _startlasernode "/Script/Escape.TableGameLaserController"))
  (bind _sequenceplayer (`LevelSequenceActor.SequencePlayer` _introsequence))
  ;[1 1 1] Enter TableGameMode
  (`Controller.SetIgnoreMoveInput` _returnvalue_2 true)
  (`Controller.SetIgnoreLookInput` _returnvalue_2 true)
  (if (`self.PlayIntro`)
    (if (`KismetSystemLibrary.IsValid` _startlasernode)
      (if (`KismetSystemLibrary.IsValid` _returnvalue_3)
        (if (> (`TableGameLaserController.CurrentActivationDuration` _returnvalue_3) 0.0)
          (`PlayerController.SetViewTargetWithBlend` (`GameplayStatics.GetPlayerController` 0) (`self.IntoSequenceCamera`) (`self.TransitionDuration`) "VTBlend_EaseInOut" 3.0 false)
          (`KismetSystemLibrary.Delay` (- (`self.TransitionDuration`) 1.0))
          (`MovieSceneSequencePlayer.Play` _sequenceplayer)
          (`KismetSystemLibrary.Delay` (- (`TimeManagementBlueprintLibrary.Conv_QualifiedFrameTimeToSeconds` (`MovieSceneSequencePlayer.GetDuration` (`LevelSequenceActor.SequencePlayer` _introsequence))) 1.0))
          (`MovieSceneSequencePlayer.Pause` _sequenceplayer)
          (set `self.PlayIntro` false)))))
  (`PlayerController.SetViewTargetWithBlend` (`GameplayStatics.GetPlayerController` 0) self (`self.TransitionDuration`) "VTBlend_EaseInOut" 3.0 false)
  (`KismetSystemLibrary.Delay` (`self.TransitionDuration`))
  (`self.EnableInput` _returnvalue)
  (set `PlayerController.bShowMouseCursor` true _returnvalue)
  (bind _asfp_controller_adv (cast `/Game/EscapeCustomAssets/Blueprints/FP_Controller_Adv` (`GameplayStatics.GetPlayerController` 0)))
  (`/Game/EscapeCustomAssets/Blueprints/FP_Controller_Adv.OnSwitchHighlightMethod` _asfp_controller_adv "NewEnumerator0")
  (set `self.InTableView` true))

(event `Key|RightMouseButton`
  (params (Key :type "Key Structure"))
  (bind _returnvalue (`GameplayStatics.GetPlayerController` 0))
  ;[1 1 1] Exit TableGameMode
  (:`Pressed`
    (if (`self.InTableView`)
      (set `self.InTableView` false)
      (set `PlayerController.bShowMouseCursor` false (`GameplayStatics.GetPlayerController` 0))
      (`PlayerController.SetViewTargetWithBlend` (`GameplayStatics.GetPlayerController` 0) (`GameplayStatics.GetPlayerCharacter` 0) (`self.TransitionDuration`) "VTBlend_EaseInOut" 3.0 false)
      (`KismetSystemLibrary.Delay` (`self.TransitionDuration`))
      (bind _asfp_controller_adv (cast `/Game/EscapeCustomAssets/Blueprints/FP_Controller_Adv` (`GameplayStatics.GetPlayerController` 0)))
      (`/Game/EscapeCustomAssets/Blueprints/FP_Controller_Adv.OnSwitchHighlightMethod` _asfp_controller_adv "NewEnumerator1")
      (`Controller.ResetIgnoreMoveInput` _returnvalue)
      (`Controller.ResetIgnoreLookInput` _returnvalue))))

(fn `UserConstructionScript`)