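; TableGameFloor is an actor that runs a short camera cutscene when play begins, temporarily taking the view away from the player.
; A timeline's first event track blends the view to this actor with an ease-in-out curve and locks move and look input.
; Its second blends back to the player character, then restores input after a delay matching the shared transition duration.
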(event `self.ReceiveBeginPlay`
  (bind _returnvalue (`GameplayStatics.GetPlayerController` 0))
  (bind _returnvalue_2 (`GameplayStatics.GetPlayerController` 0))
  (`Timeline|Timeline_0`
    (:`NewTrack_0`
      (`PlayerController.SetViewTargetWithBlend` (`GameplayStatics.GetPlayerController` 0) self (`self.TransitionDuration`) "VTBlend_EaseInOut" 3.0 false)
      (`Controller.SetIgnoreMoveInput` _returnvalue_2 true)
      (`Controller.SetIgnoreLookInput` _returnvalue_2 true))
    (:`NewTrack_1`
      (`PlayerController.SetViewTargetWithBlend` (`GameplayStatics.GetPlayerController` 0) (`GameplayStatics.GetPlayerCharacter` 0) (`self.TransitionDuration`) "VTBlend_EaseInOut" 3.0 false)
      (`KismetSystemLibrary.Delay` (`self.TransitionDuration`))
      (`Controller.ResetIgnoreMoveInput` _returnvalue)
      (`Controller.ResetIgnoreLookInput` _returnvalue))))

(fn `UserConstructionScript`)